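; Projectile actor that flies forward at a set Speed and expires on a timer, with no overlap or hit response in its graph.
; Tick offsets the root along its forward vector without sweeping and accumulates lifetime.
; After ten seconds it disables capsule collision, cuts the spot light and spawns the ShotHitEffect system once via the Hit flag.
; The point light then fades out quickly, and the still-moving actor destroys itself a few seconds later.
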(event EventBeginPlay)

(event Collision|EventActorBeginOverlap
  (params (OtherActor :type Actor%20Object%20Reference)))

(event EventTick
  (params (DeltaSeconds :type Float%20%28single-precision%29))
  (bind _defaultsceneroot (Variables|Default|GetDefaultSceneRoot))
  (bind _defaultsceneroot_2 (Variables|Default|GetDefaultSceneRoot))
  (Transformation|AddWorldOffset _defaultsceneroot_2 (* (Math|Vector|GetForwardVector (Variables|/Script/Engine.SceneComponent|GetRelativeRotation _defaultsceneroot_2)) (Variables|Default|GetSpeed)) false false)
  (bind _output_get (Variables|Default|SetTime (+ DeltaSeconds (stale _output_get))))
  (if (>= _output_get 1e+01)
    (Rendering|Components|Light|SetIntensity (Variables|Default|GetPointLight) (Math|Float|Max(Float) (* (- 1.0 (/ (- _output_get 1e+01) 0.5)) 5e+03) 0.0))
    (if (stale _output_get_2)
      (if (>= _output_get 13.0)
        (Actor|DestroyActor))
      (else
        (bind _output_get_2 (Variables|Default|SetHit true))
        (Collision|SetCollisionEnabled (Variables|Default|GetCapsule) "NoCollision")
        (Rendering|Components|Light|SetIntensity (Variables|Default|GetSpotLight) 0.0)
        (Niagara|SpawnSystematLocation "/Game/Blueprints/ShotHitEffect.ShotHitEffect" (Transformation|GetWorldLocation _defaultsceneroot) (Variables|/Script/Engine.SceneComponent|GetRelativeRotation _defaultsceneroot))))))

(fn ConstructionScript)